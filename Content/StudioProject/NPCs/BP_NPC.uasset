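; BP_NPC is a work-in-progress enemy NPC that chases whatever actor enters its detection sphere.
; A state variable runs Wandering or Chasing each Tick, with sphere overlaps switching between Chase and the default state.
; Chasing uses swept world offsets toward the target until within AttackRange, but omits the ChaseSpeed applied in a duplicate debug event outside Tick.
; Wandering and attack logic are stubs, and range and collision results only print messages.
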(event OnComponentBeginOverlap(DetectionOverlapSphere)
  (params (OverlappedComponent :type Primitive%20Component%20Object%20Reference) (OtherActor :type Actor%20Object%20Reference) (OtherComp :type Primitive%20Component%20Object%20Reference) (OtherBodyIndex :type Integer) (bFromSweep :type Boolean) (SweepResult :type Hit%20Result%20Structure%20%28by%20ref%29))
  ;[1 1 1] Player Enters Overlap Radius
  (Variables|Default|SetPlayer OtherActor)
  (if (or (Utilities|Enum|Equal(Enum) (Variables|--State--|GetCurrentState) "NewEnumerator3") (Utilities|Enum|Equal(Enum) (Variables|--State--|GetCurrentState) "NewEnumerator1"))
    ;;[1 1 1] Transition To Chase State
    (Variables|--State--|SetCurrentState "NewEnumerator2")
    (Development|PrintString "PlayerEntersRange")))

(event OnComponentEndOverlap(DetectionOverlapSphere)
  (params (OverlappedComponent :type Primitive%20Component%20Object%20Reference) (OtherActor :type Actor%20Object%20Reference) (OtherComp :type Primitive%20Component%20Object%20Reference) (OtherBodyIndex :type Integer))
  ;[1 1 1] Player Leaves Overlap Radius
  (if (Utilities|Enum|Equal(Enum) (Variables|--State--|GetCurrentState) "NewEnumerator2")
    ;;[1 1 1] Transition To Default State
    (Variables|--State--|SetCurrentState (Variables|--State--|GetDefaultState))))

(event Custom|ChasingEvent
  (bind _player (Variables|Default|GetPlayer))
  ;[1 1 1] Chasing Event (So I can see variables with watches, wasn't working in functions)
  (Utilities|IsValid _player
    (:Is%20Valid
      (bind _output_get (Variables|ChaseState|SetChaseVectorToTarget (- (Transformation|GetActorLocation _player) (Transformation|GetWorldLocation (Variables|Default|GetDefaultSceneRoot)))))
      (if (< (Math|Vector|VectorLength _output_get) (Variables|ChaseState|GetAttackRange))
        (Development|PrintString "In range to Attack Now")
        (else
          ;;[1 1 1] Apply Movement
          (bind _sweephitresult (Transformation|AddActorWorldOffset (* (* (Math|Vector|Normalize _output_get) (Utilities|Time|GetWorldDeltaSeconds)) (Variables|ChaseState|GetChaseSpeed)) true))
          (Utilities|FlowControl|Sequence
            (:then_0
              ;;[1 1 1] Check for collision with obstacles
              (if (.bblockinghit _sweephitresult)
                (Development|PrintString "Oops NPC Hit Something")))
            (:then_1
              (if true
                _))))))))

(event Custom|EnterAttackState
  (CallFunction|AttackState))

(event Custom|AttackState
  (if true
    _))

(event Custom|ExitAttackState
  (CallFunction|EnterChasingEvent))

(event Custom|ExecuteAttackAction)

(event Custom|EnterChasingEvent
  (CallFunction|ChasingEvent))

(event EventBeginPlay
  ;[1 1 1] Set Starting State
  (Variables|--State--|SetCurrentState (Variables|--State--|GetDefaultState)))

(event EventTick
  (params (DeltaSeconds :type Float%20%28single-precision%29))
  ;[1 1 1] Every Frame
  ;;[1 1 1] Select State
  (switch Utilities|FlowControl|Switch|SwitchonE_NPC_States (Variables|--State--|GetCurrentState)
    (:NewEnumerator1
      (CallFunction|Wandering))
    (:NewEnumerator2
      (CallFunction|Chasing))))

(fn ConstructionScript)

(fn SelectBehaviour)

(fn Wandering)

(fn Chasing
  (bind _player (Variables|Default|GetPlayer))
  (Utilities|IsValid _player
    (:Is%20Valid
      (bind _output_get (Variables|ChaseState|SetChaseVectorToTarget (- (Transformation|GetActorLocation _player) (Transformation|GetWorldLocation (Variables|Default|GetDefaultSceneRoot)))))
      (if (< (Math|Vector|VectorLength _output_get) (Variables|ChaseState|GetAttackRange))
        (Development|PrintString "In range to Attack Now")
        (LocalVariables|SetNewLocalVar_0 (* (Math|Vector|Normalize _output_get) (Utilities|Time|GetWorldDeltaSeconds)))
        (else
          ;[1 1 1] Apply Movement
          (bind _sweephitresult (Transformation|AddActorWorldOffset (* (Math|Vector|Normalize _output_get) (Utilities|Time|GetWorldDeltaSeconds)) true))
          ;[1 1 1] Check for collision with obstacles
          (if (.bblockinghit _sweephitresult)
            (Development|PrintString "Oops NPC Hit Something")))))))