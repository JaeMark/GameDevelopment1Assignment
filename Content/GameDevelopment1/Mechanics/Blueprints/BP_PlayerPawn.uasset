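; Player pawn for a 2D game with four-way Paper2D flipbook animation, sign reading and interaction.
; Axis input moves the capsule by swept world offsets, caches the movement vector and shows Sign text on blocking hits, hidden on overlap end.
; Each move updates animation, picking a walk flipbook by dominant axis or south-facing idle below a speed threshold.
; Interact activates overlapping interactable actors; Action A/B states are cached, while debug widget creation is disconnected.
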(event OnComponentBeginOverlap(Capsule)
  (params (OverlappedComponent :type Primitive%20Component%20Object%20Reference) (OtherActor :type Actor%20Object%20Reference) (OtherComp :type Primitive%20Component%20Object%20Reference) (OtherBodyIndex :type Integer) (bFromSweep :type Boolean) (SweepResult :type Hit%20Result%20Structure%20%28by%20ref%29)))

(event OnComponentHit(Capsule)
  (params (HitComponent :type Primitive%20Component%20Object%20Reference) (OtherActor :type Actor%20Object%20Reference) (OtherComp :type Primitive%20Component%20Object%20Reference) (NormalImpulse :type Vector :default "0, 0, 0") (Hit :type Hit%20Result%20Structure%20%28by%20ref%29)))

(event OnComponentEndOverlap(Capsule)
  (params (OverlappedComponent :type Primitive%20Component%20Object%20Reference) (OtherActor :type Actor%20Object%20Reference) (OtherComp :type Primitive%20Component%20Object%20Reference) (OtherBodyIndex :type Integer))
  (bind _assign_4 (Utilities|Casting|CastToSign_4 OtherActor))
  (Default|HideTextUI _assign_4)
  (Development|PrintString "Hide Sign"))

(event Custom|UpdateAnimationState
  (bind _currentjoystickinput (Variables|--CachedInput(State)|GetCurrentJoystickInput))
  (bind _paperflipbook (Variables|Default|GetPaperFlipbook))
  (bind _currentjoystickinput_2 (Variables|--CachedInput(State)|GetCurrentJoystickInput))
  (bind _paperflipbook_2 (Variables|Default|GetPaperFlipbook))
  ;[0 0.111 0] Calculate useful values to use later (For animation or etc).
  (Utilities|FlowControl|Sequence
    (:then_0
      ;;[0.0369 0.0246 0 1 12] Magnitude of the movement vector gives us amount of movement without direction. This is uuseful for determining which animation we should play (Walk, Idle) regardless of direction wwe are facing.
      (Variables|--EditableSettings|SetCurrentMoveSpeed (Math|Vector2D|Vector2DLength _currentjoystickinput)))
    (:then_1
      ;;[0.0369 0.0246 0 1 12] Normalized Movement Vector. This gives us direction without magnitude. It will always have a length of 1. This is uuseful anytime we need a single direction value.
      (Variables|--CachedInput(State)|SetCurrentNormalizedMovementDirection (Class|KismetMathLibrary|NormalSafe2D _currentjoystickinput 0.0)))
    (:then_2
      ;;[0.0369 0.0246 0 1 12] Are we Idle or Walking? This will get more complicated later but it's a good starting point.
      (bind _output_get (Variables|--CachedInput(State)|SetIsMoving (> (Variables|--EditableSettings|GetCurrentMoveSpeed) (* (Variables|--AnimationVariables|GetMoveAnimationSpeedThreshold) (Utilities|Time|GetWorldDeltaSeconds)))))
      ;[0 0.111 0] If we are moving in any direction faster then our threshold, we are walking, otherwise, we Idle.
      (if _output_get
        ;[0 0.111 0] Calculate which direction our Walk animation will be facing. Later on we will replace this with a Blend Tree but it's a good example/place to start.
        ;;[0 0.0369 0 1 12] Select Horizontal or Vertical. Basically we are checking if the Horizontal or Vertical component of the movement vector is larger.
        (if (< (Math|Float|Absolute(Float) (.x _currentjoystickinput_2)) (Math|Float|Absolute(Float) (.y _currentjoystickinput_2)))
          ;;[0 0.0369 0] Vertical Axis is bigger. Are we moving North or South?
          (if (> (.y (Variables|--CachedInput(State)|GetCurrentJoystickInput)) 0.0)
            ;;[0 0.0369 0] Vertical Facing Selection
            (Sprite|SetFlipbook _paperflipbook_2 (Variables|--AnimationState|GetWalkS))
            (else
              (Sprite|SetFlipbook _paperflipbook_2 (Variables|--AnimationState|GetWalkN))))
          (else
            ;;[0 0.0369 0] East/West - Horizontal Axis is longer then Vertical
            (if (> (.x (Variables|--CachedInput(State)|GetCurrentJoystickInput)) 0.0)
              ;;[0 0.0369 0] Horizontal Move
              (Sprite|SetFlipbook _paperflipbook (Variables|--AnimationState|GetWalkW))
              (else
                (Sprite|SetFlipbook _paperflipbook (Variables|--AnimationState|GetWalkE))))))
        (else
          ;;[1 0.25 0] Idle - Currently this always sets the Idle facing South. How would you fix this to face the last facing direction?
          (Sprite|SetFlipbook (Variables|Default|GetPaperFlipbook) (Variables|--AnimationState|GetIdleS)))))))

(event EventBeginPlay
  ;[1 0.25 0] Note: This is currently set up to require an Object of GD_PlayerBasePawn_1 to work (since we need to be able to access its cached input variables for the binding to work). There are better ways to deal with this in more general ways so we don't have to create a new Debug UI every time we use a different pawn.
)

(event Collision|EventActorBeginOverlap
  (params (OtherActor :type Actor%20Object%20Reference)))

(event EventTick
  (params (DeltaSeconds :type Float%20%28single-precision%29)))

(event Collision|EventHit
  (params (MyComp :type Primitive%20Component%20Object%20Reference) (Other :type Actor%20Object%20Reference) (OtherComp :type Primitive%20Component%20Object%20Reference) (bSelfMoved :type Boolean) (HitLocation :type Vector :default "0, 0, 0") (HitNormal :type Vector :default "0, 0, 0") (NormalImpulse :type Vector :default "0, 0, 0") (Hit :type Hit%20Result%20Structure%20%28by%20ref%29))
  ;[1 0.25 0] Debugging Message for Any Collision (Incoming or outgoing)
  (if (Variables|DEBUGGING|GetDEBUG_MODE)
    (Development|PrintString (Utilities|String|Append (Utilities|GetDisplayName MyComp) (Utilities|GetDisplayName Other)) true true "(R=0.000000,G=0.660000,B=1.000000,A=1.000000)" 1e+02)))

(event Input|ActionEvents|InputActionActionA
  (params (Key :type Key%20Structure :default "None"))
  ;[0 0.0369 0] Cache Action Inputs
  (:Pressed
    (Variables|--CachedInput(State)|SetInput_ActionA true))
  (:Released
    (Variables|--CachedInput(State)|SetInput_ActionA false)))

(event Input|ActionEvents|InputActionActionB
  (params (Key :type Key%20Structure :default "None"))
  ;[0 0.0369 0] Cache Action Inputs
  (:Pressed
    (Variables|--CachedInput(State)|SetInput_ActionB true))
  (:Released
    (Variables|--CachedInput(State)|SetInput_ActionB false)))

(event Input|ActionEvents|InputActionInteract
  (params (Key :type Key%20Structure :default "None"))
  ;[0 0.111 0] Interact Event
  (:Pressed
    ;;[0 0.0369 0 1 14] Activate any InteractableActors within overlap range.
    (for _array_element (Collision|GetOverlappingActors (Variables|Default|GetCapsule) "/Game/GDWeeks/GD_Week5/BP_GDInteractableActor_5.BP_GDInteractableActor_5_C" :!class /Script/Engine.PrimitiveComponent)
      (bind _asbp_gdinteractable_actor_5 (Utilities|Casting|CastToBP_GDInteractableActor_5 _array_element)
        (:then
          (Default|ActivateInteraction _asbp_gdinteractable_actor_5))
        (:CastFailed
          ;[0.22 0 0 1 12] Shouldnt ever be called but I was curious if it would be.
          (Development|PrintString "Overlap found other Actors" true true "(R=1.000000,G=0.000000,B=0.128810,A=1.000000)" 1e+01))))))

(event Input|AxisEvents|InputAxisHorizontal
  (params (AxisValue :type Float%20%28single-precision%29))
  (bind _movespeed (Variables|--EditableSettings|GetMoveSpeed))
  ;[0 0.111 0 1 24] Input and Movement 01
  ;;[0 0.0369 0] Cache Joystick Input in Vector2D, with speed
  ;;;[0 1 0 1 14] We don't have a velocity (since we are not using forces) so we need to track this outselves
  (bind _output_get (Variables|--CachedInput(State)|SetCurrentJoystickInput (Math|Vector2D|MakeVector2D (* AxisValue _movespeed) (* (stale Input|AxisEvents|InputAxisVertical AxisValue) _movespeed))))
  ;;[0 0.0369 0] PlayerMovement
  (bind _sweephitresult (Transformation|AddWorldOffset (Variables|Default|GetCapsule) (Math|Vector|MakeVector (.x _output_get) (.y _output_get) 0.0) true false))
  ;;[0 0.0369 0] Update Animation
  (CallFunction|UpdateAnimationState)
  ;[0 0.369 0.369] Sign Collisions (We will make this more general later on)
  (if (.bBlockingHit (Collision|BreakHitResult _sweephitresult))
    (bind _assign_4 (Utilities|Casting|CastToSign_4 (.HitActor (Collision|BreakHitResult _sweephitresult))))
    (Default|ShowTextUI _assign_4)))

(event Input|AxisEvents|InputAxisVertical
  (params (AxisValue :type Float%20%28single-precision%29))
  (bind _movespeed (Variables|--EditableSettings|GetMoveSpeed))
  ;[0 0.111 0 1 24] Input and Movement 01
  ;;[0 0.0369 0] Cache Joystick Input in Vector2D, with speed
  ;;;[0 1 0 1 14] We don't have a velocity (since we are not using forces) so we need to track this outselves
  (bind _output_get (Variables|--CachedInput(State)|SetCurrentJoystickInput (Math|Vector2D|MakeVector2D (* (stale Input|AxisEvents|InputAxisHorizontal AxisValue) _movespeed) (* AxisValue _movespeed))))
  ;;[0 0.0369 0] PlayerMovement
  (bind _sweephitresult (Transformation|AddWorldOffset (Variables|Default|GetCapsule) (Math|Vector|MakeVector (.x _output_get) (.y _output_get) 0.0) true false))
  ;;[0 0.0369 0] Update Animation
  (CallFunction|UpdateAnimationState)
  ;[0 0.369 0.369] Sign Collisions (We will make this more general later on)
  (if (.bBlockingHit (Collision|BreakHitResult _sweephitresult))
    (bind _assign_4 (Utilities|Casting|CastToSign_4 (.HitActor (Collision|BreakHitResult _sweephitresult))))
    (Default|ShowTextUI _assign_4)))

(fn ConstructionScript)