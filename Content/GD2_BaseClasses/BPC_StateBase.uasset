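; BPC_StateBase is a base state component that tracks an actor's health and alive state.
; TakeDamage lowers health, clamped at zero, then runs CheckForDeath, which calls Death to clear IsAlive but never returns true for DeathBlow.
; HealDamage only returns the capped healed value without storing it, while Revive sets capped health and restores IsAlive.
; A DEBUGMODE flag gates the printed damage and death messages.
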(event EventBeginPlay)

(event EventTick
  (params (DeltaSeconds :type Float%20%28single-precision%29)))

(fn TakeDamage
  (params (DamageToTake :type Integer))
  (bind _output_get (Variables|--StateHealth|SetCurrentHealth (Math|Integer|Max(Integer) (- (Variables|--StateHealth|GetCurrentHealth) DamageToTake))))
  (bind _isdead (CallFunction|CheckforDeath))
  (if (Variables|Default|GetDEBUG_MODE)
    (Development|PrintString (Utilities|String|Append "In Take Damage: " "Took Damage:  " (Utilities|String|ToString(Integer) DamageToTake) "" " Remaining Health: " "" "Is Dead")))
  (return _output_get _isdead))

(fn HealDamage
  (params (HealAmount :type Integer))
  (return (Math|Integer|Min(Integer) (+ HealAmount (Variables|--StateHealth|GetCurrentHealth)) (Variables|--StateHealth|GetMaxHealth))))

(fn CheckforDeath
  (if (< (Variables|--StateHealth|GetCurrentHealth) 1)
    ;[1 1 1] Applies Death State
    (CallFunction|Death)
    ;[1 1 1] This is all Debug.Log(Actor.name + " has died)
    (if (Variables|Default|GetDEBUG_MODE)
      (Utilities|FlowControl|Sequence
        (:then_0
          (Development|PrintString (Utilities|String|Append (Utilities|GetDisplayName (Components|GetOwner)) " has Died! Tragic!")))
        (:then_1
          (return false)))
      (else
        (return false)))))

(fn Death
  (Variables|--StateHealth|SetIsAlive false)
  (if (Variables|Default|GetDEBUG_MODE)
    ;[1 1 1] All just a single debug message
    (Development|PrintString (Utilities|String|Append (Utilities|GetDisplayName (Components|GetOwner)) " is now dead! The End!")))
  (return))

(fn Revive
  (params (AmountOfHealthToRestore :type Integer))
  (bind _output_get (Variables|--StateHealth|SetCurrentHealth (Math|Integer|Min(Integer) AmountOfHealthToRestore (Variables|--StateHealth|GetMaxHealth))))
  (bind _output_get_2 (Variables|--StateHealth|SetIsAlive true))
  (return _output_get_2 _output_get))