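; BPC_InteractionBase is a base component for interactions, implementing an attack that damages a target and a cooldown timer.
; ActivateInteractionAbility checks the passed object for a valid BPC_StateBase component, then calls AttackInteraction, which invokes TakeDamage on its target component.
; Tick counts the cooldown down until the interaction is ready, and InitializeAsReady sets it ready directly.
; Activation ignores readiness, and the cooldown reset logic is disconnected.
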(event EventBeginPlay)

(event EventTick
  (params (DeltaSeconds :type Float%20%28single-precision%29))
  (CallFunction|FrameUpdateforCooldownTimers DeltaSeconds))

(fn FrameUpdateforCooldownTimers
  (params (DeltaTime :type Float%20%28single-precision%29))
  (if (not (Variables|--State|GetInteractionIsReady))
    (bind _output_get (Variables|--State|SetCurrentInteractCooldownTime (- (Variables|--State|GetCurrentInteractCooldownTime) DeltaTime)))
    (Variables|--State|SetInteractionIsReady (< _output_get 0.0))))

(fn InitializeasReady
  (Variables|--State|SetInteractionIsReady true))

(fn ActivateInteractionAbility
  (params (NewParam :type Actor%20Object%20Reference))
  (if (Utilities|IsValid (Actor|GetComponentbyClass NewParam "/Game/GD2_BaseClasses/BPC_StateBase.BPC_StateBase_C"))
    (CallFunction|AttackInteraction 0 (Variables|--Attack|GetAttackInteraction_Damage))))

(fn AttackInteraction
  (params (TargetComponent :type BPC%20State%20Base%20Object%20Reference) (DamageToDeal :type Integer))
  (Default|TakeDamage TargetComponent DamageToDeal))