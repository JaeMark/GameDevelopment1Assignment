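; Base interactable actor that shows a notification alert and flags the player as in range while something overlaps it.
; Begin and end overlap toggle NotificationAlert visibility and IsPlayerInRange without filtering for the player; the alert starts hidden on BeginPlay.
; ActivateInteraction only prints a debug message to confirm the parent-class event is reached, and begin overlap also prints the overlapping actor's name.
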(event Custom|ActivateInteraction
  ;[1 0.25 0] Debug to see if parent class event is being called
  (Development|PrintString "In Interactable" true true "(R=0.000000,G=0.660000,B=1.000000,A=1.000000)" 3e+01))

(event EventBeginPlay
  ;[0 0.0369 0] Hide Notification on start
  (Rendering|SetVisibility (Variables|Default|GetNotificationAlert) false false))

(event Collision|EventActorBeginOverlap
  (params (OtherActor :type Actor%20Object%20Reference))
  (Utilities|FlowControl|Sequence
    (:then_0
      ;[1 0.25 0] Debugging
      (Development|PrintString (Utilities|GetDisplayName OtherActor)))
    (:then_1
      (Rendering|SetVisibility (Variables|Default|GetNotificationAlert) true false)
      (Variables|--State|SetIsPlayerInRange true))))

(event EventTick
  (params (DeltaSeconds :type Float%20%28single-precision%29)))

(event Collision|EventActorEndOverlap
  (params (OtherActor :type Actor%20Object%20Reference))
  (Rendering|SetVisibility (Variables|Default|GetNotificationAlert) false false)
  (Variables|--State|SetIsPlayerInRange false))

(fn ConstructionScript)