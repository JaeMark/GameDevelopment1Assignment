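; BP_Sign_6 is an interactable sign that shows its text in a UI panel when the player activates it.
; It extends a parent interaction Blueprint, calling the parent's events before adding its own behavior.
; Activation passes SignText to a UI call that opens the sign panel, and any actor ending overlap closes it.
; The begin-overlap override only forwards to the parent and is marked as removable.
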(event EventBeginPlay
  (|CallParentFunction))

(event Collision|EventActorBeginOverlap
  (params (OtherActor :type Actor%20Object%20Reference))
  ;[0.77 0.5133 0 1 14] Not being used and could be removed (I'll leave it in for now for demonstration purposes)
  (|CallParentFunction OtherActor))

(event EventTick
  (params (DeltaSeconds :type Float%20%28single-precision%29))
  (|CallParentFunction DeltaSeconds) ; This node is disabled and will not be called.\nDrag off pins to build functionality.
)

(event EventActivateInteraction
  ;[0 0.0369 0] Now successfully calls both parent and child event.
  (|CallParentFunction)
  (Default|CallUIOpenSignPanel (Variables|Default|GetSignText)))

(event Collision|EventActorEndOverlap
  (params (OtherActor :type Actor%20Object%20Reference))
  ;[0 0.0369 0] EndOverlap with parent event call
  (|CallParentFunction OtherActor)
  (Default|CallUICloseSignPanel))

(fn ConstructionScript
  (|CallParentFunction))