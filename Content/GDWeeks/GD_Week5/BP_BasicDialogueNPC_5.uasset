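; Dialogue NPC Blueprint that steps through a list of text lines each time the player interacts with it.
; ActivateInteraction calls the parent, then sends the NPC name, sprite and current line to the UI panel and advances the index.
; When lines run out or an actor's overlap ends, it resets the index and closes the panel.
; BeginOverlap only calls the parent, and a world-state toggle is left unconnected.
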(event EventBeginPlay
  (|CallParentFunction))

(event Collision|EventActorBeginOverlap
  (params (OtherActor :type Actor%20Object%20Reference))
  ;[0.77 0.5133 0 1 14] Not being used and could be removed (I'll leave it in for now for demonstration purposes)
  (|CallParentFunction OtherActor))

(event EventTick
  (params (DeltaSeconds :type Float%20%28single-precision%29))
  (|CallParentFunction DeltaSeconds) ; This node is disabled and will not be called.\nDrag off pins to build functionality.
)

(event EventActivateInteraction
  (bind _npc_dialoguetext (Variables|Default|GetNPC_DialogueText))
  ;[0 0.0369 0] Now successfully calls both parent and child event.
  (|CallParentFunction)
  ;;[0 0.0369 0 1 14] Is there more to say?
  (if (> (Utilities|Array|Length _npc_dialoguetext) (Variables|Default|GetCurrentDialogue_Index))
    ;;[0 0.0369 0 1 14] Get the next Text (and other Data) and pass it to the UI
    (Default|CallUIOpenNPCPanel (Variables|Default|GetNPC_Name) (Utilities|Array|Get(acopy) _npc_dialoguetext (Variables|Default|GetCurrentDialogue_Index)) (Variables|Default|GetNPC_Sprite))
    ;;[0 0.0369 0 1 14] Increment for next time.
    (Variables|Default|SetCurrentDialogue_Index (+ (Variables|Default|GetCurrentDialogue_Index) 1))
    (else
      ;[0 0.0369 0] EndOverlap with parent event call
      ;;[0 0.369 0.369 1 14] Reset for next time.
      (Variables|Default|SetCurrentDialogue_Index 0)
      (Default|CallUICloseNPCPanel))))

(event Collision|EventActorEndOverlap
  (params (OtherActor :type Actor%20Object%20Reference))
  ;[0 0.0369 0] EndOverlap with parent event call
  (|CallParentFunction OtherActor)
  ;;[0 0.369 0.369 1 14] Reset for next time.
  (Variables|Default|SetCurrentDialogue_Index 0)
  (Default|CallUICloseNPCPanel))

(fn ConstructionScript
  (|CallParentFunction))